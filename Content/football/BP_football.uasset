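; BP_football is a kickable football actor that player 0 can pass short or kick long.
; Any actor overlap enables that player's input on the ball, and ending an overlap disables it.
; While input is enabled, S and L apply PassSpeed or LongKick as a mass-independent impulse along the player controller's forward vector.
; Each kick prints a debug message on screen.
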(event Collision|EventActorBeginOverlap
  (params (OtherActor :type Actor%20Object%20Reference))
  (Input|EnableInput (Game|GetPlayerController 0)))

(event Collision|EventActorEndOverlap
  (params (OtherActor :type Actor%20Object%20Reference))
  (Input|DisableInput (Game|GetPlayerController 0)))

(event Input|KeyboardEvents|L
  (params (Key :type Key%20Structure :default "None"))
  (:Pressed
    (Physics|AddImpulse (Variables|Default|GetFootball) (* (Transformation|GetActorForwardVector (Game|GetPlayerController 0)) (Variables|Default|GetLongKick)) "None" true)
    (Development|PrintString "Long kick!" true true "(R=0.108586,G=0.000000,B=0.972595,A=1.000000)")))

(event Input|KeyboardEvents|S
  (params (Key :type Key%20Structure :default "None"))
  (:Pressed
    (Physics|AddImpulse (Variables|Default|GetFootball) (* (Transformation|GetActorForwardVector (Game|GetPlayerController 0)) (Variables|Default|GetPassSpeed)) "None" true)
    (Development|PrintString "short kick!" true true "(R=0.108586,G=0.000000,B=0.972595,A=1.000000)")))

(fn ConstructionScript)