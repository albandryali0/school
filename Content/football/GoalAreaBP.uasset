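; Football goal area that counts goals and shows score and win text through the player's ThirdPersonCharacter.
; Box overlaps pass a DoOnce, then increment Goals for BP_football; exactly five sets the win text, plays a sound and clears the text after a delay.
; DoOnce resets only in that win branch, so other overlaps leave it closed.
; Box1 overlaps copy Goals to the score text; ball-reset logic is unconnected.
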(event OnComponentBeginOverlap(Box)
  (params (OverlappedComponent :type Primitive%20Component%20Object%20Reference) (OtherActor :type Actor%20Object%20Reference) (OtherComp :type Primitive%20Component%20Object%20Reference) (OtherBodyIndex :type Integer) (bFromSweep :type Boolean) (SweepResult :type Hit%20Result%20Structure%20%28by%20ref%29))
  (Utilities|FlowControl|DoOnce false :!label _label
    (:Completed
      (bind _asbp_football (Utilities|Casting|CastToBP_football OtherActor))
      (bind _output_get (Variables|Default|Setgoals (+ (Variables|Default|Getgoals) 1)))
      (if (== (Variables|Default|Getgoals) (Variables|Default|Get5))
        (bind _asthird_person_character (Utilities|Casting|CastToThirdPersonCharacter (Game|GetPlayerCharacter 0)))
        (Variables|/Game/ThirdPersonBP/Player/ThirdPersonCharacter.ThirdPersonCharacter_C|Setgoaltext _asthird_person_character "you won !")
        (Audio|PlaySound2D "/Game/audio/anees/الدور_الثاني_Cue.الدور_الثاني_Cue" 1.0 1.0 0.0 0 0)
        (Development|PrintString (Utilities|String|ToString(Integer) _output_get) true true "(R=1.000000,G=0.847798,B=0.378222,A=1.000000)")
        (Utilities|FlowControl|Delay 5.0)
        (Variables|/Game/ThirdPersonBP/Player/ThirdPersonCharacter.ThirdPersonCharacter_C|Setgoaltext _asthird_person_character "")
        (goto _label Reset)
        (else
          (bind _asthird_person_character_2 (Utilities|Casting|CastToThirdPersonCharacter (Game|GetPlayerCharacter 0)))
          (Variables|/Game/ThirdPersonBP/Player/ThirdPersonCharacter.ThirdPersonCharacter_C|Setgoaltext _asthird_person_character_2 ""))))))

(event OnComponentBeginOverlap(Box1)
  (params (OverlappedComponent :type Primitive%20Component%20Object%20Reference) (OtherActor :type Actor%20Object%20Reference) (OtherComp :type Primitive%20Component%20Object%20Reference) (OtherBodyIndex :type Integer) (bFromSweep :type Boolean) (SweepResult :type Hit%20Result%20Structure%20%28by%20ref%29))
  (bind _asthird_person_character (Utilities|Casting|CastToThirdPersonCharacter (Game|GetPlayerCharacter 0)))
  (Variables|/Game/ThirdPersonBP/Player/ThirdPersonCharacter.ThirdPersonCharacter_C|Setfootballscore _asthird_person_character (Utilities|Text|ToText(Integer) (Variables|Default|Getgoals))))

(fn ConstructionScript)